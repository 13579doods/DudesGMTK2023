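; Player controller that lets the player click a ControllableBP actor in the world to possess it.
; BeginPlay shows the mouse cursor and adds the IMC_Controllable Enhanced Input mapping context.
; Left click runs a debug-drawn visibility trace from the deprojected cursor, then stores and possesses any ControllableBP hit.
; A raw S key event calls MoveDown on the stored controllable.
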(event EventBeginPlay
  (Variables|Default|SetbShowMouseCursor true)
  (bind _asplayer_controller (Utilities|Casting|CastToPlayerController self))
  (Utilities|IsValid (PlayerController|LocalPlayerSubsystems|GetEnhancedInputLocalPlayerSubsystem _asplayer_controller)
    (:Is%20Valid
      (Input|AddMappingContext (PlayerController|LocalPlayerSubsystems|GetEnhancedInputLocalPlayerSubsystem _asplayer_controller) "/Game/Input/IMC_Controllable.IMC_Controllable" 0 "(bIgnoreAllPressedKeysUntilRelease=True,bForceImmediately=False)"))))

(event EventTick
  (params (DeltaSeconds :type Float%20%28single-precision%29)))

(event Input|MouseEvents|LeftMouseButton
  (params (Key :type Key%20Structure :default "None"))
  (bind (_worldlocation _worlddirection) (Game|Player|ConvertMouseLocationToWorldSpace))
  (:Pressed
    (bind (_outhit _returnvalue) (Collision|LineTraceByChannel _worldlocation (+ _worldlocation (* _worlddirection 5e+03)) "TraceTypeQuery1" false 0 "ForDuration"))
    (if _returnvalue
      (bind _ascontrollable_bp (Utilities|Casting|CastToControllableBP (.HitActor (Collision|BreakHitResult _outhit))))
      (bind _output_get (Variables|Default|SetAttachedControllable _ascontrollable_bp))
      (Pawn|Possess _output_get))))

(event Input|KeyboardEvents|S
  (params (Key :type Key%20Structure :default "None"))
  (bind _attachedcontrollable (Variables|Default|GetAttachedControllable))
  (:Pressed
    (Utilities|IsValid _attachedcontrollable
      (:Is%20Valid
        (Default|MoveDown _attachedcontrollable)))))

(fn ConstructionScript)