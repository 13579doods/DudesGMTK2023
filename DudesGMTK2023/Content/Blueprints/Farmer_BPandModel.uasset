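; Farmer character Blueprint that wanders the level as a simple patrolling AI, starting when play begins.
; A recursive Patrol event sets a slow walk speed and moves to a random reachable point within a radius of the world origin.
; Each successful arrival triggers a short random pause before the next move.
; The loop stops when IsInspecting is set or a move fails, with no restart in this graph.
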(event Custom|Patrol
  (params (Patrol%20Point :type Vector) (Radius :type Float%20%28single-precision%29))
  (if (not (Variables|Default|GetIsInspecting))
    (Variables|/Script/Engine.CharacterMovementComponent|SetMaxWalkSpeed (Variables|Character|GetCharacterMovement) 2e+02)
    (AI|AIMoveTo self (.RandomLocation (AI|Navigation|GetRandomReachablePointinRadius Patrol%20Point Radius 0 0)) 0 5.0 false
      (:OnSuccess
        (Utilities|FlowControl|Delay (Math|Random|RandomFloatinRange 0.0 5.0))
        (CallFunction|Patrol Patrol%20Point Radius)))))

(event EventBeginPlay
  (CallFunction|Patrol "0, 0, 0" 2e+03))

(fn ConstructionScript)