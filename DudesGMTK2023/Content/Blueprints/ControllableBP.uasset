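; Controllable pawn Blueprint that moves on fixed world axes through Enhanced Input.
; IA_Move feeds AddMovementInput along world +X and -Y, scaled by a Speed variable.
; InitInput and ReleaseInput add and remove the IMC_Controllable mapping context on the controlling PlayerController, with no call to either in this graph.
; A disconnected copy of the InitInput logic remains in the EventGraph and never runs.
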(event Input|EnhancedActionEvents|EnhancedInputActionIA_Move
  (params (ActionValue :type Vector%202D%20Structure) (ElapsedSeconds :type Float%20%28double-precision%29) (TriggeredSeconds :type Float%20%28double-precision%29) (InputAction :type Input%20Action%20Object%20Reference :default "/Game/Input/Actions/IA_Move.IA_Move"))
  (:Triggered
    (Pawn|Input|AddMovementInput "1.000000,0.000000,0.000000" (* (.x ActionValue) (Variables|Default|GetSpeed)) false)
    (Pawn|Input|AddMovementInput "0.000000,-1.000000,0.000000" (* (.y ActionValue) (Variables|Default|GetSpeed)) false)))

(event EventTick
  (params (DeltaSeconds :type Float%20%28single-precision%29)))

(event Collision|EventActorBeginOverlap
  (params (OtherActor :type Actor%20Object%20Reference)))

(fn ConstructionScript)

(fn InitInput
  (bind _asplayer_controller (Utilities|Casting|CastToPlayerController (Pawn|GetController)))
  (Utilities|IsValid (PlayerController|LocalPlayerSubsystems|GetEnhancedInputLocalPlayerSubsystem _asplayer_controller)
    (:Is%20Valid
      (Input|AddMappingContext (PlayerController|LocalPlayerSubsystems|GetEnhancedInputLocalPlayerSubsystem _asplayer_controller) "/Game/Input/IMC_Controllable.IMC_Controllable" 0 "(bIgnoreAllPressedKeysUntilRelease=True,bForceImmediately=False)"))))

(fn ReleaseInput
  (bind _asplayer_controller (Utilities|Casting|CastToPlayerController (Pawn|GetController)))
  (Utilities|IsValid (PlayerController|LocalPlayerSubsystems|GetEnhancedInputLocalPlayerSubsystem _asplayer_controller)
    (:Is%20Valid
      (Input|RemoveMappingContext (PlayerController|LocalPlayerSubsystems|GetEnhancedInputLocalPlayerSubsystem _asplayer_controller) "/Game/Input/IMC_Controllable.IMC_Controllable" "(bIgnoreAllPressedKeysUntilRelease=True,bForceImmediately=False)"))))