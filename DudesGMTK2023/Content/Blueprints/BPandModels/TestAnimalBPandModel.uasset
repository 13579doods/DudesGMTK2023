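; Test animal Blueprint that triggers the farmer's investigate behaviour at its own location when T is pressed.
; On BeginPlay it caches the first Farmer_BP in the level.
; T flags the farmer as inspecting, sets his walk speed and AI-moves him to a random reachable point nearby.
; On arrival he patrols that area, then resumes a wide patrol around world origin after a delay unless re-alerted, or immediately if the move fails.
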(event EventBeginPlay
  (bind _outactors (Actor|GetAllActorsOfClass "/Game/Blueprints/Farmer_BP.Farmer_BP_C"))
  (Variables|Default|SetFarmer (Utilities|Array|Get(acopy) _outactors)))

(event Input|KeyboardEvents|T
  (params (Key :type Key%20Structure :default "None"))
  (bind _farmer (Variables|Default|GetFarmer))
  (bind _farmer_2 (Variables|Default|GetFarmer))
  (:Pressed
    (Variables|/Game/Blueprints/Farmer_BP.Farmer_BP_C|SetIsInspecting (Variables|Default|GetFarmer) true)
    (bind _output_get (Variables|Default|SetDestination (Transformation|GetActorLocation)))
    (Variables|/Script/Engine.CharacterMovementComponent|SetMaxWalkSpeed (Variables|/Script/Engine.Character|GetCharacterMovement _farmer) 6e+02)
    (Development|PrintString "STOP RIGHT THERE YOU CRIMINAL SCUM!!!")
    (AI|AIMoveTo _farmer (.RandomLocation (AI|Navigation|GetRandomReachablePointinRadius _output_get 2e+02 0 0)) 0 2e+02 false
      (:OnSuccess
        (Variables|/Game/Blueprints/Farmer_BP.Farmer_BP_C|SetIsInspecting _farmer_2 false)
        (Default|Patrol _farmer_2 (Variables|Default|GetDestination) 2e+02)
        (Utilities|FlowControl|Delay 1e+01)
        (if (not (Variables|/Game/Blueprints/Farmer_BP.Farmer_BP_C|GetIsInspecting _farmer_2))
          (Development|PrintString "Must've been the wind...")
          (Default|Patrol (Variables|Default|GetFarmer) "0, 0, 0" 2e+03 :!label _label)))
      (:OnFail
        (goto _label)))))

(fn ConstructionScript
  (|CallParentFunction))