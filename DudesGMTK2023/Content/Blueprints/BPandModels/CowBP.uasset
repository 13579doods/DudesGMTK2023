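; Cow Blueprint that tracks the animal's behavior state (idle, walk, eat) as Cow gameplay tags in a tag container.
; Tick sets Walk and cancels the timer while velocity is non-zero, and prints the tags for debugging.
; On stopping, Idle replaces Walk and a short timer switches it to Eat.
; BeginPlay's initial Idle starts no timer; Attack is only ever cleared here.
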(event Custom|IdleTimer
  (bind _tagcontainer (Variables|Default|GetTagContainer))
  (GameplayTags|RemoveGameplayTag _tagcontainer "(TagName=\"Cow.Idle\")" :!class /Script/GameplayTags.BlueprintGameplayTagLibrary)
  (GameplayTags|AddGameplayTag _tagcontainer "(TagName=\"Cow.Eat\")" :!class /Script/GameplayTags.BlueprintGameplayTagLibrary))

(event Collision|EventActorBeginOverlap
  (params (OtherActor :type Actor%20Object%20Reference))
  (|CallParentFunction OtherActor) ; This node is disabled and will not be called.\nDrag off pins to build functionality.
)

(event EventTick
  (params (DeltaSeconds :type Float%20%28single-precision%29))
  (bind _tagcontainer (Variables|Default|GetTagContainer))
  (Development|PrintString (GameplayTags|GetDebugStringfromGameplayTagContainer (Variables|Default|GetTagContainer)) true true "(R=0.000000,G=0.660000,B=1.000000,A=1.000000)" 0.0)
  (if (> (Math|Vector|VectorLength (Transformation|GetVelocity)) 0.0)
    (CallFunction|ClearContainer)
    (GameplayTags|AddGameplayTag _tagcontainer "(TagName=\"Cow.Walk\")" :!class /Script/GameplayTags.BlueprintGameplayTagLibrary)
    (Utilities|Time|ClearandInvalidateTimerbyHandle (Variables|Default|GetTimerHadler))
    (else
      (GameplayTags|RemoveGameplayTag _tagcontainer "(TagName=\"Cow.Walk\")" :!class /Script/GameplayTags.BlueprintGameplayTagLibrary)
      (bind _idleadded (CallFunction|AddIdleifEmpty))
      (if _idleadded
        (bind _returnvalue (Utilities|Time|SetTimerbyEvent (delegate Custom|IdleTimer) 3.0))
        (Variables|Default|SetTimerHadler _returnvalue)))))

(event EventBeginPlay
  (CallFunction|AddIdleifEmpty))

(fn ConstructionScript
  (|CallParentFunction))

(fn AddIdleifEmpty
  (bind _tagcontainer (Variables|Default|GetTagContainer))
  (if (Utilities|Array|IsEmpty (GameplayTags|BreakGameplayTagContainer _tagcontainer))
    (GameplayTags|AddGameplayTag _tagcontainer "(TagName=\"Cow.Idle\")" :!class /Script/GameplayTags.BlueprintGameplayTagLibrary)
    (return true)
    (else
      (return false))))

(fn ClearContainer
  (bind _tagcontainer (Variables|Default|GetTagContainer))
  (GameplayTags|RemoveGameplayTag _tagcontainer "(TagName=\"Cow.Attack\")" :!class /Script/GameplayTags.BlueprintGameplayTagLibrary)
  (GameplayTags|RemoveGameplayTag _tagcontainer "(TagName=\"Cow.Eat\")" :!class /Script/GameplayTags.BlueprintGameplayTagLibrary)
  (GameplayTags|RemoveGameplayTag _tagcontainer "(TagName=\"Cow.Idle\")" :!class /Script/GameplayTags.BlueprintGameplayTagLibrary)
  (GameplayTags|RemoveGameplayTag _tagcontainer "(TagName=\"Cow.Walk\")" :!class /Script/GameplayTags.BlueprintGameplayTagLibrary))