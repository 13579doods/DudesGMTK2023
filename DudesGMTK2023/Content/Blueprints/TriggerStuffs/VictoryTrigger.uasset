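; VictoryTrigger is a trigger actor that wins the game once the player has spent enough time inside it.
; Collision overlap events track whether a ControllableBP is in the volume.
; Tick accumulates time while it is inside, without resetting on exit, and calls Win on GameModeBP every tick that the total exceeds TimeToVictory.
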(event OnComponentBeginOverlap(CollisionComponent)
  (params (OverlappedComponent :type Primitive%20Component%20Object%20Reference) (OtherActor :type Actor%20Object%20Reference) (OtherComp :type Primitive%20Component%20Object%20Reference) (OtherBodyIndex :type Integer) (bFromSweep :type Boolean) (SweepResult :type Hit%20Result%20Structure%20%28by%20ref%29))
  (Utilities|Casting|CastToControllableBP OtherActor)
  (Variables|Default|SetPlayerInTrigger true))

(event OnComponentEndOverlap(CollisionComponent)
  (params (OverlappedComponent :type Primitive%20Component%20Object%20Reference) (OtherActor :type Actor%20Object%20Reference) (OtherComp :type Primitive%20Component%20Object%20Reference) (OtherBodyIndex :type Integer))
  (Utilities|Casting|CastToControllableBP OtherActor)
  (Variables|Default|SetPlayerInTrigger false))

(event EventBeginPlay)

(event EventTick
  (params (DeltaSeconds :type Float%20%28single-precision%29))
  (if (Variables|Default|GetPlayerInTrigger)
    (Variables|Default|SetConditionOutput (+ DeltaSeconds (Variables|Default|GetConditionOutput)))
    (if (> (Variables|Default|GetConditionOutput) (Variables|Default|GetTimeToVictory))
      (bind _asgame_mode_bp (Utilities|Casting|CastToGameModeBP (Game|GetGameMode)))
      (Default|Win _asgame_mode_bp))))

(fn ConstructionScript)