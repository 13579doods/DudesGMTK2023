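; Player controller that lets the player click a ControllableBP in the world to possess it.
; It shows the mouse cursor, and a left click line-traces along the deprojected cursor ray on the Visibility channel.
; A ControllableBP hit is stored as AttachedControllable and possessed.
; Possess and UnPossess events tell that pawn to initialise or release its own input.
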(event EventBeginPlay
  (Variables|Default|SetbShowMouseCursor true))

(event EventPossess
  (params (PossessedPawn :type Pawn%20Object%20Reference))
  (bind _ascontrollable_bp (Utilities|Casting|CastToControllableBP PossessedPawn))
  (Default|InitInput _ascontrollable_bp))

(event EventUnPossess
  (params (UnpossessedPawn :type Pawn%20Object%20Reference))
  (bind _ascontrollable_bp (Utilities|Casting|CastToControllableBP UnpossessedPawn))
  (Default|ReleaseInput _ascontrollable_bp))

(event Input|MouseEvents|LeftMouseButton
  (params (Key :type Key%20Structure :default "None"))
  (bind (_worldlocation _worlddirection) (Game|Player|ConvertMouseLocationToWorldSpace))
  (:Pressed
    (bind (_outhit _returnvalue) (Collision|LineTraceByChannel _worldlocation (+ _worldlocation (* _worlddirection 5e+03)) "TraceTypeQuery1" false 0 "None"))
    (if _returnvalue
      (bind _ascontrollable_bp (Utilities|Casting|CastToControllableBP (.HitActor (Collision|BreakHitResult _outhit))))
      (bind _output_get (Variables|Default|SetAttachedControllable _ascontrollable_bp))
      (Pawn|Possess _output_get))))

(fn ConstructionScript)